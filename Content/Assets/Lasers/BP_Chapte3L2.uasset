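; BP_Chapte3L2 is a laser source, apparently for Chapter 3 Level 2, that spawns its beam actor when play begins.
; BeginPlay clears SpawnReference, stores its display name as ID, and spawns a Chapter3Level2Laser at the Arrow's location with the actor's rotation.
; The spawned laser receives LaserColor and the empty SpawnReference, then joins the ChildLaser array.
; The construction script only calls its parent.
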(event EventBeginPlay
  (Variables|Default|SetSpawnReference 0)
  (Variables|Default|SetID (Utilities|GetDisplayName self))
  (Game|SpawnActorfromClass "/Game/Assets/Lasers/Chapter3Level2Laser.Chapter3Level2Laser_C" (Math|Transform|MakeTransform (Transformation|GetWorldLocation (Variables|Default|GetArrow)) (Transformation|GetActorRotation) "1.000000,1.000000,1.000000") "Undefined" "MultiplyWithRoot" 0 (Variables|Default|GetLaserColor) (Variables|Default|GetSpawnReference) 0)
  (Utilities|Array|Add (Variables|Default|GetChildLaser) 0))

(fn ConstructionScript
  (|CallParentFunction))