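; Laser puzzle target that opens a door when a BP_Laser overlaps its trigger.
; The overlap latches LaserHit, and Tick drives MoveComponentTo to lower the door from its closed height, with no reset in this graph.
; Separately, LaserBounce stores the hit response in ActiveLaser and calls PuzzleSolved, which tints a dynamic M_Solid material with the laser's color or grey.
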(event OnComponentBeginOverlap(Trigger)
  (params (OverlappedComponent :type Primitive%20Component%20Object%20Reference) (OtherActor :type Actor%20Object%20Reference) (OtherComp :type Primitive%20Component%20Object%20Reference) (OtherBodyIndex :type Integer) (bFromSweep :type Boolean) (SweepResult :type Hit%20Result%20Structure%20%28by%20ref%29))
  (Utilities|Casting|CastToBP_Laser OtherActor)
  (Development|PrintString "door open")
  (Variables|Default|SetLaserHit true))

(event EventBeginPlay)

(event EventTick
  (params (DeltaSeconds :type Float%20%28single-precision%29))
  (if (Variables|Default|GetLaserHit)
    (Components|MoveComponentTo (Variables|Default|GetDoor) "0.000000,0.000000,-1200.000000" "0.000000,90.000000,0.000000" false false 0.2 false)
    (else
      (Components|MoveComponentTo (Variables|Default|GetDoor) "0.000000,0.000000,-480.000000" "0.000000,90.000000,0.000000" false false 0.2 false))))

(fn ConstructionScript
  (|CallParentFunction))

(fn PuzzleSolved
  (params (ColorLaser :type Linear%20Color%20Structure))
  (bind _returnvalue (Rendering|Material|CreateDynamicMaterialInstance (Variables|Default|GetParent) 0 "/Game/LevelPrototyping/Materials/M_Solid.M_Solid" "None" :!class /Script/Engine.PrimitiveComponent))
  (Rendering|Material|SetVectorParameterValue _returnvalue "Base Color" (Math|Color|SelectColor ColorLaser "(R=0.317708,G=0.317708,B=0.317708,A=1.000000)" (Variables|Default|GetActiveLaser)) :!class /Script/Engine.MaterialInstanceDynamic))

(fn LaserBounce
  (params (P-LaserHit :type BP%20Laser%20Object%20Reference) (HitResponse :type Boolean) (P-HitInfomation :type Hit%20Result%20Structure))
  (Variables|Default|SetActiveLaser HitResponse)
  (CallFunction|PuzzleSolved (Variables|/Game/Assets/Lasers/BP_LaserParent.BP_LaserParent_C|GetLaserColor P-LaserHit))
  (return 0))