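; Laser puzzle target that takes on the color of the laser hitting it and turns grey when inactive.
; LaserBounce stores the hit response as the active flag and passes the laser's color to PuzzleSolved.
; PuzzleSolved prints a debug string and creates a fresh M_Solid dynamic material on each call to set the color.
; No color matching or further puzzle logic runs here.
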(event EventBeginPlay)

(fn ConstructionScript
  (|CallParentFunction))

(fn PuzzleSolved
  (params (ColorLaser :type Linear%20Color%20Structure))
  (Development|PrintString "Hello")
  (bind _returnvalue (Rendering|Material|CreateDynamicMaterialInstance (Variables|Default|GetParent) 0 "/Game/LevelPrototyping/Materials/M_Solid.M_Solid" "None" :!class /Script/Engine.PrimitiveComponent))
  (Rendering|Material|SetVectorParameterValue _returnvalue "Base Color" (Math|Color|SelectColor ColorLaser "(R=0.317708,G=0.317708,B=0.317708,A=1.000000)" (Variables|Default|GetActiveLaser)) :!class /Script/Engine.MaterialInstanceDynamic))

(fn LaserBounce
  (params (P-LaserHit :type BP%20Laser%20Object%20Reference) (HitResponse :type Boolean) (P-HitInfomation :type Hit%20Result%20Structure))
  (Variables|Default|SetActiveLaser HitResponse)
  (CallFunction|PuzzleSolved (Variables|/Game/Assets/Lasers/BP_LaserParent.BP_LaserParent_C|GetLaserColor P-LaserHit))
  (return 0))