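; Laser beam actor that tints itself with LaserColor and acts as a death trigger for BP_EstrixCharacter.
; Each tick it box-traces along its up vector and scales the beam to the blocking hit or maximum range.
; It tracks the last hit actor, sending hit or lost-hit messages through BPI_Lasers for bouncing.
; Character overlap with the trigger removes all players and opens Level2FINAL.
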(event OnComponentBeginOverlap(Trigger)
  (params (OverlappedComponent :type Primitive%20Component%20Object%20Reference) (OtherActor :type Actor%20Object%20Reference) (OtherComp :type Primitive%20Component%20Object%20Reference) (OtherBodyIndex :type Integer) (bFromSweep :type Boolean) (SweepResult :type Hit%20Result%20Structure%20%28by%20ref%29))
  ;[1 1 1] Laser Death Trigger
  (Utilities|Casting|CastToBP_EstrixCharacter OtherActor)
  (Development|PrintString "laser trigger")
  (Class|MyBlueprintFunctionLibrary|RemoveAllPlayers)
  (Game|OpenLevel(byObjectReference) "/Game/Gooie_Levels/Chapter1/Level2-FINAL.Level2-FINAL"))

(event OnComponentEndOverlap(Trigger)
  (params (OverlappedComponent :type Primitive%20Component%20Object%20Reference) (OtherActor :type Actor%20Object%20Reference) (OtherComp :type Primitive%20Component%20Object%20Reference) (OtherBodyIndex :type Integer))
  (Utilities|Casting|CastToBP_EstrixCharacter OtherActor)
  (Development|PrintString "Hello"))

(event EventBeginPlay
  (CallFunction|ChangeColor))

(event EventTick
  (params (DeltaSeconds :type Float%20%28single-precision%29))
  (CallFunction|SetEndpoint))

(fn ConstructionScript
  (|CallParentFunction))

(fn ChangeColor
  (bind _returnvalue (Rendering|Material|CreateDynamicMaterialInstance (Variables|Default|GetParent) 0 "/Game/Assets/Lasers/M_Laser.M_Laser" "None" :!class /Script/Engine.PrimitiveComponent))
  (Rendering|Material|SetVectorParameterValue _returnvalue "Color" (Variables|Default|GetLaserColor) :!class /Script/Engine.MaterialInstanceDynamic))

(fn SetEndpoint
  (bind _returnvalue (Transformation|GetActorLocation))
  (bind _returnvalue_2 (Transformation|GetActorUpVector))
  (bind _returnvalue_3 (* _returnvalue_2 2.0))
  (bind _returnvalue_4 (+ _returnvalue _returnvalue_3))
  (bind _outhit (Collision|BoxTraceByChannel _returnvalue_4 (+ _returnvalue_4 (* _returnvalue_2 (LocalVariables|GetL-Range))) "0.500000,0.500000,0.500000" "0, 0, 0" "TraceTypeQuery1" false 0 "None"))
  (bind _output_get (LocalVariables|SetL-HitInfomation _outhit))
  (LocalVariables|SetL-HitActor (.HitActor (Collision|BreakHitResult _output_get)))
  (Transformation|SetWorldScale3D (Variables|Default|GetParent) (Math|Vector|MakeVector 0.1 0.1 (Math|Float|SelectFloat (/ (+ (.Distance (Collision|BreakHitResult _output_get)) 1.0) 1e+02) (/ (LocalVariables|GetL-Range) 1e+02) (.bBlockingHit (Collision|BreakHitResult _output_get)))))
  (Utilities|FlowControl|Sequence
    (:then_0
      (if (!= (Variables|Default|GetLastHitActor) (LocalVariables|GetL-HitActor))
        (if (Utilities|DoesObjectImplementInterface (Variables|Default|GetLastHitActor) "/Game/Assets/Lasers/BPI_Lasers.BPI_Lasers_C")
          (Class|BPILasers|LaserBounce(Message) (Variables|Default|GetLastHitActor) self false (LocalVariables|GetL-HitInfomation)))
        (elif (Utilities|DoesObjectImplementInterface (LocalVariables|GetL-HitActor) "/Game/Assets/Lasers/BPI_Lasers.BPI_Lasers_C")
          (Class|BPILasers|LaserBounce(Message) (LocalVariables|GetL-HitActor) self true (LocalVariables|GetL-HitInfomation)))))
    (:then_1
      (bind _l_hitactor (LocalVariables|GetL-HitActor)
        (:then
          (Variables|Default|SetLastHitActor _l_hitactor))
        (:else)))))