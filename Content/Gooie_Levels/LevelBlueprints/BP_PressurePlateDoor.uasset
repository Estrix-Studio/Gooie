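; BP_PressurePlateDoor is a pressure plate that opens a pair of sliding doors when a GlooObject rests on it.
; Trigger overlaps play timelines that lower or raise the Button, set the ButtonTrigger flag and, on press, play a sound.
; While the flag is true, Tick repeatedly calls MoveComponentTo to slide DoorLeft and DoorRight apart.
; Releasing the plate clears the flag but has no logic to close the doors.
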(event OnComponentBeginOverlap(Trigger)
  (params (OverlappedComponent :type Primitive%20Component%20Object%20Reference) (OtherActor :type Actor%20Object%20Reference) (OtherComp :type Primitive%20Component%20Object%20Reference) (OtherBodyIndex :type Integer) (bFromSweep :type Boolean) (SweepResult :type Hit%20Result%20Structure%20%28by%20ref%29))
  (Utilities|Casting|CastToGlooObject OtherActor)
  (Audio|PlaySoundatLocation "/Engine/EditorSounds/Notifications/CompileSuccess.CompileSuccess" "0, 0, 0" "0, 0, 0" 1.0 1.0 0.0 0 0 0 0)
  (Development|PrintString "Button Press")
  (bind _plateanimation (Timeline|PlateAnimation Play)
    (:Update
      (Transformation|SetRelativeLocation (Variables|Default|GetButton) (Math|Vector|MakeVector 0.0 0.0 (Math|Float|Lerp 6.66 0.0 _plateanimation)) false false)
      (Variables|Default|SetButtonTrigger true))))

(event OnComponentEndOverlap(Trigger)
  (params (OverlappedComponent :type Primitive%20Component%20Object%20Reference) (OtherActor :type Actor%20Object%20Reference) (OtherComp :type Primitive%20Component%20Object%20Reference) (OtherBodyIndex :type Integer))
  (Utilities|Casting|CastToGlooObject OtherActor)
  (bind _plateanimation (Timeline|ReversePlate Play)
    (:Update
      (Transformation|SetRelativeLocation (Variables|Default|GetButton) (Math|Vector|MakeVector 0.0 0.0 (Math|Float|Lerp 0.0 6.66 _plateanimation)) false false)
      (Variables|Default|SetButtonTrigger false))))

(event EventTick
  (params (DeltaSeconds :type Float%20%28single-precision%29))
  (if (Variables|Default|GetButtonTrigger)
    (Utilities|FlowControl|Sequence
      (:then_0
        (Components|MoveComponentTo (Variables|Default|GetDoorLeft) "300.000000,-999.000000,0.000000" "0.000000,180.000000,0.000000" true false 0.8 false))
      (:then_1
        (Components|MoveComponentTo (Variables|Default|GetDoorRight) "300.000000,999.000000,0.000000" "0.000000,180.000000,0.000000" true false 0.8 false)))))

(fn ConstructionScript)